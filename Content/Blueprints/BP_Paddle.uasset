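; BP_Paddle is a player-controlled paddle that slides horizontally along the X axis.
; The MoveRight axis input offsets PaddleSprite by the axis value times PaddleSpeed, without sweeping or delta-time scaling.
; Tick then checks the actor's location and snaps X back within hardcoded left and right limits, keeping Y and Z unchanged.
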(event `InputAxis|MoveRight`
  (params (AxisValue :type "Float (single-precision)"))
  (`SceneComponent.K2_AddWorldOffset` (`self.PaddleSprite`) (* (1.0 0.0 0.0) (* AxisValue (`self.PaddleSpeed`))) false false))

(event `self.ReceiveTick`
  (params (DeltaSeconds :type "Float (single-precision)"))
  (bind (_returnvalue_x _returnvalue_y _returnvalue_z) (`KismetMathLibrary.BreakVector` (`self.K2_GetActorLocation`)))
  (if (> _returnvalue_x 1470.0)
    (`self.K2_SetActorLocation` (`KismetMathLibrary.MakeVector` 1470.0 _returnvalue_y _returnvalue_z))
    (elif (< _returnvalue_x -1440.0)
      (`self.K2_SetActorLocation` (`KismetMathLibrary.MakeVector` -1440.0 _returnvalue_y _returnvalue_z)))))

(fn `UserConstructionScript`)