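; BP_Ball is a ball actor that destroys any BP_Brick it hits, as in a brick-breaker game.
; On BeginPlay it records the capsule's world Y position, then rewrites that Y every Tick to keep movement in the X-Z plane.
; The capsule's hit event casts the other actor to BP_Brick and destroys it on success.
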(event `self.ReceiveBeginPlay`
  (set `self.InitialY` (.y (`SceneComponent.K2_GetComponentLocation` (`self.Capsule`)))))

(event `self.ReceiveTick`
  (params (DeltaSeconds :type "Float (single-precision)"))
  ;[1 1 1] Disable ball moving in z-axis
  (`SceneComponent.K2_SetWorldLocation` (`self.Capsule`) (`KismetMathLibrary.MakeVector` (.x (`SceneComponent.K2_GetComponentLocation` (`self.Capsule`))) (`self.InitialY`) (.z (`SceneComponent.K2_GetComponentLocation` (`self.Capsule`)))) false false))

(event `self.Capsule.OnComponentHit`
  (params (HitComponent :type "PrimitiveComponent Object Reference") (OtherActor :type "Actor Object Reference") (OtherComp :type "PrimitiveComponent Object Reference") (NormalImpulse :type "Vector Structure") (Hit :type "HitResult Structure (by ref)"))
  (bind _asbp_brick (cast `/Game/Blueprints/BP_Brick` OtherActor))
  (`self.K2_DestroyActor` _asbp_brick))

(fn `UserConstructionScript`)