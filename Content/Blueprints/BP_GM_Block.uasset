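; BP_GM_Block is the game mode for a brick-breaker game, tracking lives and remaining bricks.
; On BeginPlay it sets the starting lives and counts the BP_Brick actors in the level.
; CheckLives decrements lives, then respawns BP_Ball or prints game over, while CheckBricks decrements bricks and prints completion at zero.
; StartGame switches to game-only input and unpauses the game.
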(event `self.ReceiveBeginPlay`
  ;[1 1 1] Comment
  (`|ExecutionSequence`
    (:`then_1`
      ;;[1 1 1] Comment
      (set `self.Lives` 3))
    (:`then_2`
      (bind _outactors (`GameplayStatics.GetAllActorsOfClass` "/Game/Blueprints/BP_Brick.BP_Brick_C"))
      (set `self.Bricks` (`KismetArrayLibrary.Array_Length` _outactors)))))

(event `/Game/Blueprints/BPI_Block.CheckLives`
  (bind _result (`/Engine/EditorBlueprintResources/StandardMacros.DecrementInt` (`self.Lives`))
    (:`  `
      (if (> _result 0)
        (`|SpawnActorFromClass` "/Game/Blueprints/BP_Ball.BP_Ball_C" (`KismetMathLibrary.MakeTransform` (0.0 0.0 1080.0)) "Undefined" "OverrideRootScale" null null)
        (`KismetSystemLibrary.PrintString` (`KismetStringLibrary.Conv_IntToString` _result))
        (else
          (`KismetSystemLibrary.PrintString` "Game Over"))))))

(event `/Game/Blueprints/BPI_Block.CheckBricks`
  (bind _result (`/Engine/EditorBlueprintResources/StandardMacros.DecrementInt` (`self.Bricks`))
    (:`  `
      (if (== _result 0)
        (`KismetSystemLibrary.PrintString` "Game Completed")
        (else
          (`KismetSystemLibrary.PrintString` (`KismetStringLibrary.Conv_IntToString` _result)))))))

(event `/Game/Blueprints/BPI_Block.StartGame`
  (`WidgetBlueprintLibrary.SetInputMode_GameOnly` (`GameplayStatics.GetPlayerController` 0))
  (`GameplayStatics.SetGamePaused` false))

(fn `UserConstructionScript`)