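; BP_Collectable is a falling Paper2D pickup that the paddle catches, apparently a coin in a block game.
; Tick moves the sprite straight down at a constant, frame-rate-independent speed without sweeping.
; Overlapping BP_Paddle calls CheckCoinsMessage on the BP_GM_Block game mode cached at BeginPlay, then destroys the actor.
; An uncaught pickup destroys itself after a short delay.
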(event `self.ReceiveBeginPlay`
  (`|ExecutionSequence`
    (:`then_0`
      (bind _asbp_gm_block (cast `/Game/Blueprints/BP_GM_Block` (`GameplayStatics.GetGameMode`)))
      (set `self.REF_GameMode` _asbp_gm_block))
    (:`then_1`
      (`KismetSystemLibrary.Delay` 3.0)
      (`self.K2_DestroyActor`))))

(event `self.ReceiveActorBeginOverlap`
  (params (OtherActor :type "Actor Object Reference"))
  (cast `/Game/Blueprints/BP_Paddle` OtherActor)
  (message `/Game/Blueprints/BPI_Block.CheckCoins` (`self.REF_GameMode`))
  (`self.K2_DestroyActor`))

(event `self.ReceiveTick`
  (params (DeltaSeconds :type "Float (single-precision)"))
  (`SceneComponent.K2_AddWorldOffset` (`self.PaperSprite`) (* (0.0 0.0 -1.0) (* DeltaSeconds 1000.0)) false false))

(fn `UserConstructionScript`)